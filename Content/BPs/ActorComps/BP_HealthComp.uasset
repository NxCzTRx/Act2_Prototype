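; BP_HealthComp is an actor component that tracks integer health for its owning actor.
; On BeginPlay it sets current health to the maximum.
; SubtractHealth reduces current health by the damage taken, clamped between zero and the maximum, and IsAlive reports whether any health remains.
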(event EventBeginPlay
  (Variables|Default|SetCurrentHealth (Variables|Default|GetMaxHealth)))

(fn IsAlive
  (return (> (Variables|Default|GetCurrentHealth) 0)))

(fn SubtractHealth
  (params (DamageTaken :type Integer))
  (Variables|Default|SetCurrentHealth (Math|Integer|Clamp(Integer) (- (Variables|Default|GetCurrentHealth) DamageTaken) 0 (Variables|Default|GetMaxHealth))))