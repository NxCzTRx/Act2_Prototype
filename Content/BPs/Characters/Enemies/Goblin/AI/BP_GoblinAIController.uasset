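; AI controller for the goblin enemy that runs BT_Goblin and feeds it the player as Target, a current state and a point of interest.
; Perception updates are split by sight, hearing and damage, then written to the blackboard as enum state changes.
; Sighting the player sets the seen state, while losing sight stores the last known location and switches state.
; Noise or damage does likewise with the stimulus location, unless already in the seen state.
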(event OnTargetPerceptionUpdated(AIPerception)
  (params (Actor :type Actor%20Object%20Reference) (Stimulus :type AI%20Stimulus%20Structure))
  (bind _stimuluslocation (Utilities|Struct|BreakAIStimulus Stimulus))
  (Utilities|FlowControl|Sequence
    (:then_0
      (bind (_result _state) (CallFunction|CanSenseSomething "/Script/AIModule.AISense_Sight" Stimulus))
      (if _result
        (if _state
          (CallFunction|OnActorSeen Actor)
          (else
            (CallFunction|OnActorLost _stimuluslocation Actor)))))
    (:then_1
      (bind (_result_2 _state_2) (CallFunction|CanSenseSomething "/Script/AIModule.AISense_Hearing" Stimulus))
      (if _result_2
        (if _state_2
          (CallFunction|OnDamageorHear _stimuluslocation :!label _label))))
    (:then_2
      (bind (_result_3 _state_3) (CallFunction|CanSenseSomething "/Script/AIModule.AISense_Damage" Stimulus))
      (if _result_3
        (if _state_3
          (goto _label))))))

(event EventBeginPlay
  (AI|RunBehaviorTree "/Game/BPs/Characters/Enemies/Goblin/AI/BT_Goblin.BT_Goblin")
  (AI|Components|Blackboard|SetValueasObject (AI|GetBlackboard 0) (Utilities|Name|MakeLiteralName "Target") (Game|GetPlayerCharacter 0))
  (CallFunction|SetKeyCurrentState (Utilities|Enum|LiteralenumBPE_EnemyStates "NewEnumerator0")))

(event EventSetKeyCurrentState
  (params (NewState :type BPE_EnemyStates%20Enum :default "NewEnumerator0"))
  (AI|Components|Blackboard|SetValueasEnum (AI|GetBlackboard 0) (Utilities|Name|MakeLiteralName "CurrentState") NewState))

(fn ConstructionScript)

(fn CanSenseSomething
  (params (SenseType :type Object%20Class%20Reference) (Stimulus :type AI%20Stimulus%20Structure))
  (bind _returnvalue (Class|AIPerceptionSystem|GetSenseClassforStimulus Stimulus))
  (return (== _returnvalue SenseType) (.bSuccessfullySensed (Utilities|Struct|BreakAIStimulus Stimulus))))

(fn OnActorSeen
  (params (Actor :type Object%20Object%20Reference))
  (if (== Actor (Game|GetPlayerCharacter 0))
    (CallFunction|SetKeyCurrentState "NewEnumerator1")))

(fn OnActorLost
  (params (LastKnownLocation :type Vector) (Actor :type Object%20Object%20Reference))
  (if (== Actor (Game|GetPlayerCharacter 0))
    (AI|Components|Blackboard|SetValueasVector (AI|GetBlackboard 0) (Utilities|Name|MakeLiteralName "PointOfInterest") LastKnownLocation)
    (CallFunction|SetKeyCurrentState "NewEnumerator2")))

(fn OnDamageorHear
  (params (PointOfInterest :type Vector))
  (bind _returnvalue (AI|GetBlackboard 0))
  (if (!= (Math|Byte|MakeLiteralByte (Class|BlackboardComponent|GetValueasEnum _returnvalue (Utilities|Name|MakeLiteralName "CurrentState"))) (Math|Byte|MakeLiteralByte (Utilities|Enum|LiteralenumBPE_EnemyStates "NewEnumerator1")))
    (AI|Components|Blackboard|SetValueasVector _returnvalue (Utilities|Name|MakeLiteralName "PointOfInterest") PointOfInterest)
    (CallFunction|SetKeyCurrentState "NewEnumerator2")))