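; BP_Goblin is a goblin enemy character that patrols, yells before combat and attacks damageable targets.
; Events play attack and yell montages, switch movement between idle, walk and run speeds, and route damage to a health component, destroying the actor on death.
; ExecuteDamage box-overlaps pawns in AttackArea and damages them through the BPI_DamageableByEnemy interface.
; Helper functions cycle looping PatrolPath points and report combat readiness, set once the yell montage starts.
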(event EventAttack
  (Animation|Montage|PlayMontage (Variables|Character|GetMesh) "/Game/BPs/Characters/Enemies/Goblin/Anim/Animations/AM_Goblin_Attack.AM_Goblin_Attack"))

(event EventSetNewSpeed
  (params (NewSpeed :type BPE_EnemySpeeds%20Enum :default "NewEnumerator0"))
  (Variables|/Script/Engine.CharacterMovementComponent|SetMaxWalkSpeed (Variables|Character|GetCharacterMovement) (Utilities|Select :Index NewSpeed :NewEnumerator0 0.0 :NewEnumerator1 1.5e+02 :NewEnumerator2 4e+02)))

(event EventStopAttack
  (Animation|StopAnimMontage "/Game/BPs/Characters/Enemies/Goblin/Anim/Animations/AM_Goblin_Attack.AM_Goblin_Attack"))

(event EventScream
  (Animation|Montage|PlayMontage (Variables|Character|GetMesh) "/Game/BPs/Characters/Enemies/Goblin/Anim/Animations/AM_Goblin_Yell.AM_Goblin_Yell"
    (:then
      (Variables|Default|SetIsReady true))))

(event EventTakeDamage
  (params (DamageTaken :type Integer))
  (Default|SubtractHealth (Variables|Default|GetBP_HealthComp) DamageTaken)
  (if (not (Default|IsAlive (Variables|Default|GetBP_HealthComp)))
    (Actor|DestroyActor)))

(fn ConstructionScript)

(fn ExecuteDamage
  (bind _outactors (Collision|BoxOverlapActors (Transformation|GetWorldLocation (Variables|Default|GetAttackArea)) (Components|Box|GetScaledBoxExtent (Variables|Default|GetAttackArea)) (Utilities|Array|MakeArray "ObjectTypeQuery3") 0 :!class /Script/Engine.KismetSystemLibrary))
  (for _array_element _outactors
    (if (Utilities|DoesObjectImplementInterface _array_element "/Game/BPs/Interfaces/BPI_DamageableByEnemy.BPI_DamageableByEnemy_C")
      (Class|BPIDamageablebyEnemy|TakeDamagebyEnemy(Message) _array_element (Variables|Default|GetDamage)))))

(fn CalculateNewPatrolPoint
  (bind _output_get (Variables|Default|SetCurrentPointLocation (Default|GetLocationatIndex (Variables|Default|GetPatrolPath) (Variables|Default|GetCurrentIndex))))
  (Variables|Default|SetCurrentIndex (Math|Integer|%(Integer) (+ (Variables|Default|GetCurrentIndex) 1) (Default|GetPathLength (Variables|Default|GetPatrolPath))))
  (return _output_get))

(fn GetIsReadyforCombat
  (return (Variables|Default|GetIsReady)))