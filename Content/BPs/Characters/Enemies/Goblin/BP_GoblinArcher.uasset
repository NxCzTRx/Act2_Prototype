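; BP_GoblinArcher is a goblin archer enemy with events for attacking, screaming, speed changes and damage.
; Scream plays a yell montage and flags it combat-ready, while Attack plays the shooting montage and InstantiateArrow spawns an arrow from the bow aimed at the player.
; CalculateNewPatrolPoint cycles through PatrolPath locations, SetNewSpeed switches idle, walk or run speeds, and damage feeds the health component, destroying the actor on death.
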(event EventAttack
  (Animation|Montage|PlayMontage (Variables|Character|GetMesh) "/Game/BPs/Characters/Enemies/Goblin/Anim/Animations/AM_Goblin_ShootArrow.AM_Goblin_ShootArrow"))

(event EventSetNewSpeed
  (params (NewSpeed :type BPE_EnemySpeeds%20Enum :default "NewEnumerator0"))
  (Variables|/Script/Engine.CharacterMovementComponent|SetMaxWalkSpeed (Variables|Character|GetCharacterMovement) (Utilities|Select :Index NewSpeed :NewEnumerator0 0.0 :NewEnumerator1 1.5e+02 :NewEnumerator2 4e+02)))

(event EventStopAttack
  (Animation|StopAnimMontage "/Game/BPs/Characters/Enemies/Goblin/Anim/Animations/AM_Goblin_Attack.AM_Goblin_Attack"))

(event EventScream
  (Animation|Montage|PlayMontage (Variables|Character|GetMesh) "/Game/BPs/Characters/Enemies/Goblin/Anim/Animations/AM_Goblin_Yell.AM_Goblin_Yell"
    (:then
      (Variables|Default|SetIsReady true))))

(event EventTakeDamage
  (params (DamageTaken :type Integer))
  (Default|SubtractHealth (Variables|Default|GetBP_HealthComp) DamageTaken)
  (if (not (Default|IsAlive (Variables|Default|GetBP_HealthComp)))
    (Actor|DestroyActor)))

(fn ConstructionScript)

(fn InstantiateArrow
  (bind _bow (Variables|Default|GetBow))
  (bind _returnvalue (Transformation|GetWorldTransform _bow))
  (bind _location (Math|Transform|BreakTransform _returnvalue))
  (Game|SpawnActorfromClass "/Game/BPs/Others/BP_EnemyArrow.BP_EnemyArrow_C" (Math|Transform|MakeTransform _location (Math|Rotator|FindLookatRotation _location (Transformation|GetActorLocation (Game|GetPlayerCharacter 0)))) "Undefined" "MultiplyWithRoot" 0 0)
  (Audio|PlaySound2D "/Game/ExternalAssets/Free_Sounds_Pack/wav/Whoosh_1-1.Whoosh_1-1" 1.0 1.0 0.0 0 0))

(fn CalculateNewPatrolPoint
  (bind _output_get (Variables|Default|SetCurrentPointLocation (Default|GetLocationatIndex (Variables|Default|GetPatrolPath) (Variables|Default|GetCurrentIndex))))
  (Variables|Default|SetCurrentIndex (Math|Integer|%(Integer) (+ (Variables|Default|GetCurrentIndex) 1) (Default|GetPathLength (Variables|Default|GetPatrolPath))))
  (return _output_get))

(fn GetIsReadyforCombat
  (return (Variables|Default|GetIsReady)))