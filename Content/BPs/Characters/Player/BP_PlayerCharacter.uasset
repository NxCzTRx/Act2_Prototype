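; Player character Blueprint with camera-relative movement, look input, a melee attack and a health bar widget.
; Attacks play a montage gated by DoOnce and make noise; ExecuteDamage box-overlaps pawns, damaging those implementing BPI_DamageableByPlayer through the interface and reporting damage events for AI senses.
; Enemy damage reduces the health component and refreshes the bar, or opens the initial menu level on death.
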(event Custom|ExecuteDamage
  (bind _playerdamageattack (Variables|Default|GetPlayerDamageAttack))
  ;[1 1 1] Damage After Attack animation event
  (bind _outactors (Collision|BoxOverlapActors (Transformation|GetWorldLocation (Variables|Default|GetAttackArea)) (Components|Box|GetScaledBoxExtent (Variables|Default|GetAttackArea)) (Utilities|Array|MakeArray "ObjectTypeQuery3") 0 :!class /Script/Engine.KismetSystemLibrary))
  (for _array_element _outactors
    (if (Utilities|DoesObjectImplementInterface _array_element "/Game/BPs/Interfaces/BPI_DamageableByPlayer.BPI_DamageableByPlayer_C")
      (Class|BPIDamageablebyPlayer|TakeDamage(Message) _array_element _playerdamageattack)
      (Class|AISenseDamage|ReportDamageEvent _array_element self (Math|Conversions|ToFloat(Integer) _playerdamageattack) (Transformation|GetActorLocation) "0, 0, 0" "None")
      (Audio|PlaySound2D "/Game/ExternalAssets/Free_Sounds_Pack/wav/Stab_4-1.Stab_4-1" 1.0 1.0 0.0 0 0))))

(event Input|EnhancedActionEvents|EnhancedInputActionIA_Attack
  (params (ActionValue :type Boolean) (ElapsedSeconds :type Float%20%28double-precision%29) (TriggeredSeconds :type Float%20%28double-precision%29) (InputAction :type Input%20Action%20Object%20Reference :default "/Game/BPs/Input/IA_Attack.IA_Attack"))
  (Utilities|FlowControl|DoOnce false :!label _label
    (:Completed
      (Animation|Montage|PlayMontage (Variables|Character|GetMesh) "/Game/BPs/Characters/Player/Anim/Animations/AM_Player_Attack1.AM_Player_Attack1"
        (:then
          (Class|Actor|MakeNoise 1.0 0 (Transformation|GetActorLocation) 0.0 "None"))
        (:OnCompleted
          (goto _label Reset))))))

(event Input|EnhancedActionEvents|EnhancedInputActionIA_Move
  (params (ActionValue :type Vector%202D%20Structure) (ElapsedSeconds :type Float%20%28double-precision%29) (TriggeredSeconds :type Float%20%28double-precision%29) (InputAction :type Input%20Action%20Object%20Reference :default "/Game/BPs/Input/IA_Move.IA_Move"))
  (bind _returnvalue (Pawn|GetControlRotation :!class /Script/Engine.Pawn))
  (bind _yaw (Math|Rotator|BreakRotator _returnvalue))
  (bind _returnvalue_2 (Math|Rotator|MakeRotator 0.0 0.0 _yaw))
  ;[1 1 1] Player Movement
  (Pawn|Input|AddMovementInput (Math|Vector|GetForwardVector _returnvalue_2) (.y ActionValue) false)
  (Pawn|Input|AddMovementInput (Math|Vector|GetRightVector _returnvalue_2) (.x ActionValue) false))

(event Input|EnhancedActionEvents|EnhancedInputActionIA_Look
  (params (ActionValue :type Vector%202D%20Structure) (ElapsedSeconds :type Float%20%28double-precision%29) (TriggeredSeconds :type Float%20%28double-precision%29) (InputAction :type Input%20Action%20Object%20Reference :default "/Game/BPs/Input/IA_Look.IA_Look"))
  ;[1 1 1] Camera Movement
  (Pawn|Input|AddControllerYawInput (.x ActionValue))
  (Pawn|Input|AddControllerPitchInput (* (.y ActionValue) -1.0)))

(event EventBeginPlay
  (bind _bp_healthcomp (Variables|Default|GetBP_HealthComp))
  (bind _returnvalue (UserInterface|CreateWidget "/Game/UI/WB_HealthBar.WB_HealthBar_C"))
  (bind _output_get (Variables|Default|SetWB_HealthBar _returnvalue))
  (UserInterface|Viewport|AddtoViewport _output_get 0)
  (Default|SetHealthBar (Variables|Default|GetWB_HealthBar) (Variables|/Game/BPs/ActorComps/BP_HealthComp.BP_HealthComp_C|GetMaxHealth _bp_healthcomp) (Variables|/Game/BPs/ActorComps/BP_HealthComp.BP_HealthComp_C|GetCurrentHealth _bp_healthcomp)))

(event EventTakeDamagebyEnemy
  (params (DamageTaken :type Integer))
  (bind _bp_healthcomp (Variables|Default|GetBP_HealthComp))
  (Default|SubtractHealth (Variables|Default|GetBP_HealthComp) DamageTaken)
  (if (Default|IsAlive (Variables|Default|GetBP_HealthComp))
    (Default|SetHealthBar (Variables|Default|GetWB_HealthBar) (Variables|/Game/BPs/ActorComps/BP_HealthComp.BP_HealthComp_C|GetMaxHealth _bp_healthcomp) (Variables|/Game/BPs/ActorComps/BP_HealthComp.BP_HealthComp_C|GetCurrentHealth _bp_healthcomp))
    (else
      (Game|OpenLevel(byName) "InitialMenuMap"))))

(fn ConstructionScript)